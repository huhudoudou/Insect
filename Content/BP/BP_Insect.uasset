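; BP_Insect is an actor that shows an insect mesh through its own 2D scene capture, with UI-toggled spinning.
; On BeginPlay it limits the capture to itself, creates the WPG_Main widget and binds to its rotator click event.
; That event's flag either clears or starts a looping timer, which yaws the static mesh in small fixed steps instead of using Tick.
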(event `self.ReceiveTick`
  (params (DeltaSeconds :type "Float (single-precision)")))

(event `self.ReceiveBeginPlay`
  (bind _mainui (`self.MainUI`))
  (`|ExecutionSequence`
    (:`then_0`
      (`SceneCaptureComponent.ShowOnlyActorComponents` (`self.SceneCaptureComponent2D`) self false))
    (:`then_1`
      (bind _returnvalue (`|CreateWidget` "/Game/BP/UI/WPG_Main.WPG_Main_C"))
      (set `self.MainUI` _returnvalue)
      (`UserWidget.AddToViewport` _returnvalue 0)
      (`/Engine/EditorBlueprintResources/StandardMacros.IsValid` _mainui
        (:`Is Valid`
          (add `/Game/BP/UI/WPG_Main.OnClickRotator` _mainui (delegate `CustomEvent`)))))))

(event `CustomEvent`
  (params (`bRotator?` :type Boolean))
  (if `bRotator?`
    (`KismetSystemLibrary.K2_ClearAndInvalidateTimerHandle` (stale _returnvalue))
    (else
      (bind _returnvalue (`KismetSystemLibrary.K2_SetTimerDelegate` (delegate `CustomEvent_0`) 0.01 true)))))

(event `CustomEvent_0`
  (`SceneComponent.K2_AddRelativeRotation` (`self.StaticMesh`) (struct :`Yaw` 1.0) false false))

(fn `UserConstructionScript`)