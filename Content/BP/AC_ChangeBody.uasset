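; AC_ChangeBody is a component that swaps or clears the static meshes attached under a given scene component, likely as body parts.
; SetBody assigns a mesh to direct static mesh children whose component tag equals the index converted to a name.
; Refresh clears the mesh on those children and resets the parent's relative rotation to zero within the loop.
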(event `SetBody`
  (params (SceneComp :type "SceneComponent Object Reference") (Mesh :type "StaticMesh Object Reference") (Index :type Integer))
  (for _array_element (`SceneComponent.GetChildrenComponents` SceneComp false)
    (bind _asstatic_mesh_component (cast `StaticMeshComponent` _array_element))
    (if (`self.ComponentHasTag` _asstatic_mesh_component (`KismetStringLibrary.Conv_StringToName` (`KismetStringLibrary.Conv_IntToString` Index)))
      (`StaticMeshComponent.SetStaticMesh` _asstatic_mesh_component Mesh))))

(event `Refresh`
  (params (SceneComp :type "SceneComponent Object Reference"))
  (for _array_element (`SceneComponent.GetChildrenComponents` SceneComp false)
    (bind _asstatic_mesh_component (cast `StaticMeshComponent` _array_element))
    (`StaticMeshComponent.SetStaticMesh` _asstatic_mesh_component null)
    (`SceneComponent.K2_SetRelativeRotation` :`self` SceneComp)))