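; BP_SpectorPawn is a pawn, apparently for spectating, that hands player control over to BP_Pawn when F is pressed.
; The key press first calls StartRT(true) on a BP_Insect found in the level.
; It then shows the cached WPG_Main UI, or creates it with a reference to itself, and has player controller 0 possess a BP_Pawn found in the level.
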(event `Key|F`
  (params (Key :type "Key Structure"))
  (bind _mainui (`self.MainUI`))
  (:`Pressed`
    (`|ExecutionSequence`
      (:`then_0`
        (bind _returnvalue (`GameplayStatics.GetActorOfClass` "/Game/BP/BP_Insect.BP_Insect_C"))
        (`/Engine/EditorBlueprintResources/StandardMacros.IsValid` _returnvalue
          (:`Is Valid`
            (`/Game/BP/BP_Insect.StartRT` _returnvalue true))))
      (:`then_1`
        (`/Engine/EditorBlueprintResources/StandardMacros.IsValid` _mainui
          (:`Is Valid`
            (set `Widget.Visibility` "Visible" _mainui))
          (:`Is Not Valid`
            (bind _returnvalue_2 (`|CreateWidget` "/Game/BP/UI/WPG_Main.WPG_Main_C" null self))
            (set `self.MainUI` _returnvalue_2)
            (`UserWidget.AddToViewport` _returnvalue_2 0)))
        (bind _returnvalue_3 (`GameplayStatics.GetActorOfClass` "/Game/Core/BP_Pawn.BP_Pawn_C"))
        (`/Engine/EditorBlueprintResources/StandardMacros.IsValid` _returnvalue_3
          (:`Is Valid`
            (`Controller.Possess` (`GameplayStatics.GetPlayerController` 0) _returnvalue_3)))))))

(fn `UserConstructionScript`)