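; BP_Pawn is an input pawn for inspecting a BP_Insect actor with the mouse.
; On BeginPlay it caches the first BP_Insect in the level and enables input from player controller 0.
; Mouse X and Y apply local yaw and pitch to the insect's component, scaled by RotationSpeed.
; The wheel zooms by sliding the insect's SceneCaptureComponent2D along local X, ignoring steps outside a fixed range.
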(event `self.ReceiveBeginPlay`
  (bind _outactors (`GameplayStatics.GetAllActorsOfClass` "/Game/BP/BP_Insect.BP_Insect_C"))
  (set `self.Insect` (`|GetArrayItem` _outactors))
  (`self.EnableInput` (`GameplayStatics.GetPlayerController` 0)))

(event `InputAxisKey|MouseWheelAxis`
  (params (AxisValue :type "Float (single-precision)"))
  (bind _returnvalue (* AxisValue 0.2))
  (bind _scenecapturecomponent2d (`/Game/BP/BP_Insect.SceneCaptureComponent2D` (`self.Insect`)))
  (bind _relativelocation_x (`KismetMathLibrary.BreakVector` (`SceneComponent.RelativeLocation` _scenecapturecomponent2d)))
  (if (`KismetMathLibrary.InRange_FloatFloat` (+ _relativelocation_x _returnvalue) -45.0 -35.0)
    (`SceneComponent.K2_AddLocalOffset` _scenecapturecomponent2d (`KismetMathLibrary.MakeVector` _returnvalue) false false)))

(event `InputAxisKey|MouseX`
  (params (AxisValue :type "Float (single-precision)"))
  (`SceneComponent.K2_AddLocalRotation` (`/Game/BP/BP_Insect.Insect` (`self.Insect`)) (`KismetMathLibrary.MakeRotator` 0.0 0.0 (* AxisValue (`self.RotationSpeed`))) false false))

(event `InputAxisKey|MouseY`
  (params (AxisValue :type "Float (single-precision)"))
  (`SceneComponent.K2_AddLocalRotation` (`/Game/BP/BP_Insect.Insect` (`self.Insect`)) (`KismetMathLibrary.MakeRotator` 0.0 (* AxisValue (`self.RotationSpeed`))) false false))

(fn `UserConstructionScript`)